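; Base enemy character that handles entry and death presentation for enemies.
; On BeginPlay a reversed dissolve timeline materializes the body and equipped weapon, hiding asset loading from the player, while a random entry montage plays.
; On death it freezes animation, disables capsule collision and removes UI widgets.
; It then async-loads a Niagara effect tinted by the material's edge color, dissolves body and weapon, and destroys both.
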(event `self.ReceiveBeginPlay`
  (bind _entrymontagestoplay (`self.EntryMontagesToPlay`))
  (bind _returnvalue (`PawnCombatComponent.GetCharacterCurrentEquippedWeapon` (`self.EnemyCombatComponent`)))
  (`|ExecutionSequence`
    (:`then_0`
      ;[0.9022 0.276 1 1 16] Tricky to avoid showing the loading of the assets to the player. We use a FX to hide it
      (`TimelineComponent.SetPlayRate` (`self.EntryRestoreTimeline`) (/ 1.0 (`self.TotalEntryRestoreTime`)))
      (bind (_direction _normalizedfloattrack) (`Timeline|EntryRestoreTimeline` :!via `ReverseFromEnd`)
        (:`Update`
          (`MeshComponent.SetScalarParameterValueOnMaterials` (`self.Mesh`) "DissolveAmount" _normalizedfloattrack)
          (`/Engine/EditorBlueprintResources/StandardMacros.IsValid` _returnvalue
            (:`Is Valid`
              (`MeshComponent.SetScalarParameterValueOnMaterials` (`WBBaseWeapon.WeaponMesh` _returnvalue) "DissolveAmount" _normalizedfloattrack))))))
    (:`then_1`
      (if (`KismetArrayLibrary.Array_IsNotEmpty` _entrymontagestoplay)
        (`self.PlayAnimMontage` (`KismetArrayLibrary.Array_Random` _entrymontagestoplay))))))

(event `/Game/Blueprints/Core/Enemy/BPI_EnemyDeath.OnEnemyDied`
  (params (DissolveNiagaraSystem :type "NiagaraSystem Soft Object Reference"))
  (bind _mesh (`self.Mesh`))
  (bind _returnvalue (`PawnCombatComponent.GetCharacterCurrentEquippedWeapon` (`self.EnemyCombatComponent`)))
  (bind _returnvalue_2 (`PawnCombatComponent.GetCharacterCurrentEquippedWeapon` (`self.EnemyCombatComponent`)))
  (`|ExecutionSequence`
    (:`then_0`
      (set `SkeletalMeshComponent.bPauseAnims` true (`self.Mesh`))
      (`PrimitiveComponent.SetCollisionEnabled` (`self.CapsuleComponent`) "NoCollision"))
    (:`then_1`
      (`EnemyUIComponent.RemoveEnemyDrawnWidget` (`self.EnemyUIComponent`)))
    (:`then_2`
      (bind _object (`|LoadAsset` DissolveNiagaraSystem)
        (:`Completed`
          (bind _asniagara_system (cast `NiagaraSystem` _object))
          (bind _returnvalue_3 (`NiagaraFunctionLibrary.SpawnSystemAttached` _asniagara_system (`self.Mesh`) "None" (0.0 0.0 0.0) (struct) "KeepRelativeOffset" true))
          (bind _returnvalue_4 (`PrimitiveComponent.CreateDynamicMaterialInstance` _mesh 0 (`PrimitiveComponent.GetMaterial` _mesh 0) "None"))
          (bind _returnvalue_5 (`MaterialInstanceDynamic.K2_GetVectorParameterValue` _returnvalue_4 "DissolveEdgeColor"))
          (`NiagaraComponent.SetNiagaraVariableLinearColor` _returnvalue_3 "DissolveParticleColor" _returnvalue_5)
          (`TimelineComponent.SetPlayRate` (`self.DissolveTimeline`) (/ 1.0 (`self.TotalDissolveTime`)))
          (bind (_direction _normalizedfloattrack) (`Timeline|DissolveTimeline` :!via `PlayFromStart`)
            (:`Update`
              (`MeshComponent.SetScalarParameterValueOnMaterials` (`self.Mesh`) "DissolveAmount" _normalizedfloattrack)
              (`/Engine/EditorBlueprintResources/StandardMacros.IsValid` _returnvalue
                (:`Is Valid`
                  (`MeshComponent.SetScalarParameterValueOnMaterials` (`WBBaseWeapon.WeaponMesh` _returnvalue) "DissolveAmount" _normalizedfloattrack))))
            (:`Finished`
              (`/Engine/EditorBlueprintResources/StandardMacros.IsValid` _returnvalue_2
                (:`Is Valid`
                  (`self.K2_DestroyActor` _returnvalue_2))
                (:`Is Not Valid`
                  _))
              (`self.K2_DestroyActor`))))))))

(fn `UserConstructionScript`)