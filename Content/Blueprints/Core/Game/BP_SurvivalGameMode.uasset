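; Survival game mode Blueprint that announces incoming waves on screen.
; On BeginPlay it binds to the game mode state-change delegate and reacts only to the state that waits to spawn a new wave.
; That state creates a countdown widget, adds it to the viewport, sets its text to the current wave number and starts the countdown using the spawn wait time.
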(event `self.ReceiveBeginPlay`
  (add `self.OnSurvivalGameModeStateChangedDelegate` (delegate `OnSurvivalGameModeStateChangedDelegate_Event`)))

(event `OnSurvivalGameModeStateChangedDelegate_Event` :!signature `self.OnSurvivalGameModeStateChangedDelegate`
  (params (CurrentState :type "EWBSurvivalGameModeState Enum" :default "WaitSpawnNewWave"))
  (switch `EWBSurvivalGameModeState` CurrentState
    (:`WaitSpawnNewWave`
      (`self.CreateWaveWidgetWithCountdown` (`|FormatText` "Wave {CurrentWaveCount} Coming In" (`self.CurrentWaveCount`)) (`self.SpawnNewWaveWaitTime`)))))

(fn `CreateWaveWidgetWithCountdown`
  (params (InTextContentToDisplay :type Text) (InTotalCountdownTime :type "Float (double-precision)"))
  (bind _returnvalue (`|CreateWidget` "/Game/Blueprints/UI/Widget/GameModeWidgets/WBP_WaveTextWithCountdown.WBP_WaveTextWithCountdown_C"))
  (`UserWidget.AddToViewport` _returnvalue 0)
  (`TextBlock.SetText` (`/Game/Blueprints/UI/Widget/GameModeWidgets/WBP_WaveTextWithCountdown.TextBlock_WaveText` _returnvalue) (`local.InTextContentToDisplay`))
  (`/Game/Blueprints/UI/Widget/GameModeWidgets/WBP_WaveTextWithCountdown.StartCountdown` _returnvalue (`local.InTotalCountdownTime`)))

(fn `UserConstructionScript`)